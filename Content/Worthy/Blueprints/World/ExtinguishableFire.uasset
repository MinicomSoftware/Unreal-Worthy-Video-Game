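; ExtinguishableFire is a world hazard that hurts the player standing in it and can be put out by attacks.
; BeginPlay starts a positional fire sound, and Tick sphere-traces around its box, damaging any ThirdPersonCharacter implementing MainPlayerInterface while Health remains.
; AttackEntity reduces Health; at zero it swaps fire particles for smoke, switches sounds, then destroys the actor after a delay.
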(event EventBeginPlay
  ;[1 1 1] Create and play sound - autoloops in wav file
  (bind _returnvalue (Audio|SpawnSoundatLocation "/Game/Worthy/Sounds/firesound.firesound" (Transformation|GetWorldLocation (Variables|Default|GetBox)) "0, 0, 0" 1.0 1.0 0.0 "/Game/Worthy/Sounds/FireRadius.FireRadius" 0 false))
  (Audio|Components|Audio|Play _returnvalue 0.0))

(event Collision|EventActorBeginOverlap
  (params (OtherActor :type Actor%20Object%20Reference)))

(event EventTick
  (params (DeltaSeconds :type Float%20%28single-precision%29))
  (bind _box (Variables|Default|GetBox))
  (bind _returnvalue (Transformation|GetWorldLocation _box))
  ;[1 1 1] Damage main player if standing on the fire
  (if (> (Variables|Default|Gethealth) 0.0)
    (bind _outhit (Collision|SphereTraceForObjects _returnvalue _returnvalue 1.1e+02 (Variables|Default|GetObject%20Types) false 0 "None"))
    (if (Utilities|DoesObjectImplementInterface (.HitActor (Collision|BreakHitResult _outhit)) "/Game/Worthy/Blueprints/MainCharacter/MainPlayerInterface.MainPlayerInterface_C")
      (bind _asthird_person_character (Utilities|Casting|CastToThirdPersonCharacter (.HitActor (Collision|BreakHitResult _outhit))))
      (Default|TakeDamage _asthird_person_character 0.01))))

(event EventAttackEntity
  (params (damage :type Float%20%28single-precision%29))
  ;[1 1 1] When the player attacks the fire
  (if (> (Variables|Default|Gethealth) 0.0)
    (bind _output_get (Variables|Default|Sethealth (- (Variables|Default|Gethealth) damage)))
    (if (<= _output_get 0.0)
      (Audio|PlaySoundatLocation "/Game/Worthy/Sounds/firegone.firegone" (Transformation|GetWorldLocation (Variables|Default|GetBox)) "0, 0, 0" 0.2 1.0 0.0 "/Game/Worthy/Sounds/SphereSoundRadius.SphereSoundRadius" 0 0)
      (Audio|Components|Audio|Stop (stale EventBeginPlay _returnvalue))
      (Rendering|SetVisibility (Variables|Default|GetP_Fire_Big) false false)
      (Rendering|SetVisibility (Variables|Default|GetP_Smoke_D) true false)
      (Utilities|FlowControl|Delay 1e+01)
      (Actor|DestroyActor))))

(fn ConstructionScript)