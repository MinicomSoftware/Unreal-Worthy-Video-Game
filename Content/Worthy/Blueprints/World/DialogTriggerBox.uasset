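; DialogTriggerBox is a world trigger that shows a dialog message on the HUD when the player enters it.
; On overlap with an actor implementing MainPlayerInterface, it gets the messaging HUD reference from the GameVariables game instance and displays its configured text for a set duration.
; An optional flag destroys the trigger after it fires, making the message one-time.
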(event OnComponentBeginOverlap(CollisionComponent)
  (params (OverlappedComponent :type Primitive%20Component%20Object%20Reference) (OtherActor :type Actor%20Object%20Reference) (OtherComp :type Primitive%20Component%20Object%20Reference) (OtherBodyIndex :type Integer) (bFromSweep :type Boolean) (SweepResult :type Hit%20Result%20Structure%20%28by%20ref%29))
  ;[1 1 1] trigger
  (if (Utilities|DoesObjectImplementInterface OtherActor "/Game/Worthy/Blueprints/MainCharacter/MainPlayerInterface.MainPlayerInterface_C")
    (bind _asgame_variables (Utilities|Casting|CastToGameVariables (Game|GetGameInstance)))
    (Default|DisplayMessageXSeconds (Variables|/Game/Worthy/GameVariables.GameVariables_C|GetMessagingHUDref _asgame_variables) (Variables|Default|GetTrigger%20Box%20Dialog) (Variables|Default|GetDialog%20Duration))
    (if (Variables|Default|GetDestory%20on%20Trigger)
      (Actor|DestroyActor))))

(event EventBeginPlay)

(event Collision|EventActorBeginOverlap
  (params (OtherActor :type Actor%20Object%20Reference)))

(event EventTick
  (params (DeltaSeconds :type Float%20%28single-precision%29)))

(fn ConstructionScript)