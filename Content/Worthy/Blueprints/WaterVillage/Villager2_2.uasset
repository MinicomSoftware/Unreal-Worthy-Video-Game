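; Villager NPC for the water village that wanders to random navigable points and greets the player on interaction.
; A looping timer drives Move, which plays a run animation during AI MoveTo, then a random idle, unless set idle or non-wandering.
; Interact returns a greeting and sets a flag, so the next Move plays an interaction animation and restarts the timer at a shorter interval.
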(event Custom|move
  (bind _mesh (Variables|Character|GetMesh))
  ;[1 1 1] Random Movement
  (if (Variables|Default|GetplayerInteracted)
    ;[1 1 1] Player Interacted
    (Components|Animation|PlayAnimation (Variables|Character|GetMesh) "/Game/Wizards/Animations/InteractAnim.InteractAnim" false)
    (Utilities|FlowControl|Delay 1.8)
    (Components|Animation|PlayAnimation (Variables|Character|GetMesh) "/Game/Wizards/Animations/Idle01Anim.Idle01Anim" true)
    (Variables|Default|SetplayerInteracted false)
    (Utilities|Time|SetTimerbyEvent (delegate Custom|move) 3.0 true)
    (elif (and (not (Variables|Default|GetisIdle)) (Variables|Default|GetrandomMovement))
      (Components|Animation|PlayAnimation (Variables|Character|GetMesh) "/Game/Wizards/Animations/BattleRunForwardAnim.BattleRunForwardAnim" true)
      (AI|AIMoveTo self (.RandomLocation (Class|NavigationSystemV1|GetRandomPointinNavigableRadius (Transformation|GetActorLocation) 1e+03 0 0)) 0 5.0 false
        (:OnSuccess
          _)
        (:OnFail
          _))
      (switch int (Math|Random|RandomInteger 2)
        (:Default
          (Components|Animation|PlayAnimation _mesh "/Game/Wizards/Animations/Idle01Anim.Idle01Anim" true :!label _label))
        (:0
          (Components|Animation|PlayAnimation _mesh "/Game/Wizards/Animations/Idle02Anim.Idle02Anim" true))
        (:1
          (goto _label))))))

(event Custom|PlayIdleAnimation
  ;[1 1 1] Idle animation
  (if (Variables|Default|GetisIdle)
    (Components|Animation|PlayAnimation (Variables|Character|GetMesh) "/Game/Wizards/Animations/Idle02Anim.Idle02Anim" true)))

(event EventBeginPlay
  ;[1 1 1] Begin
  (Utilities|Time|SetTimerbyEvent (delegate Custom|move) 8.0 true)
  (CallFunction|PlayIdleAnimation))

(fn ConstructionScript)

(fn Interact
  (params (player :type Character%20Object%20Reference) (playerwidget :type User%20Widget%20Object%20Reference))
  (Variables|Default|SetplayerInteracted true)
  (return "Hello there!" 0))